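; Sample character that exercises the Corrbolg inventory component by sending gameplay-tagged action requests with instanced-struct payloads.
; On BeginPlay the server requests a load from client using the CT_Items table.
; Debug keys B and N store a random stack or retrieve one of a random sample food or drink item.
; Both paths then share a tail that saves to client and logs the inventory by item name.
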(event `self.ReceiveBeginPlay`
  (if (`KismetSystemLibrary.IsServer`)
    (bind _returnvalue (`BlueprintInstancedStructLibrary.MakeInstancedStruct` (make `CorrbolgSaveGameContextFragment` "/Game/Fragments/CT_Items.CT_Items")))
    (`CorrbolgInventoryComponent.RequestAction` (`self.ACOMP_CorrbolgSampleInventory`) (`BlueprintGameplayTagLibrary.MakeLiteralGameplayTag` (struct :`TagName` "Corrbolg.Inventory.Action.LoadFromClient")) _returnvalue)))

(event `Key|B`
  (params (Key :type "Key Structure"))
  (:`Pressed`
    (`self.StoreItem`)))

(event `Key|N`
  (params (Key :type "Key Structure"))
  (:`Pressed`
    (`self.RetrieveItem`)))

(event `StoreItem`
  (bind _returnvalue (`BlueprintInstancedStructLibrary.MakeInstancedStruct` (make `CorrbolgStorageContextFragment` (`KismetArrayLibrary.Array_Random` (`|MakeArray` "/Game/Fragments/DA_Apple.DA_Apple" "/Game/Fragments/DA_Milk.DA_Milk" "/Game/Fragments/DA_Orange.DA_Orange" "/Game/Fragments/DA_Tea.DA_Tea" :!type "CorrbolgItemDefinition Object Reference")) (`KismetMathLibrary.RandomInteger` 3))))
  (`CorrbolgInventoryComponent.RequestAction` (`self.ACOMP_CorrbolgSampleInventory`) (`BlueprintGameplayTagLibrary.MakeLiteralGameplayTag` (struct :`TagName` "Corrbolg.Inventory.Action.Store")) _returnvalue)
  (bind _returnvalue_2 (`BlueprintInstancedStructLibrary.MakeInstancedStruct` (make `CorrbolgActionContextFragment`) :!label _label))
  (`CorrbolgInventoryComponent.RequestAction` (`self.ACOMP_CorrbolgSampleInventory`) (`BlueprintGameplayTagLibrary.MakeLiteralGameplayTag` (struct :`TagName` "Corrbolg.Inventory.Action.SaveToClient")) _returnvalue_2)
  (bind _returnvalue_3 (`BlueprintInstancedStructLibrary.MakeInstancedStruct` (make `CorrbolgLogContextFragment` (struct :`TagName` "Corrbolg.UI.Item.Name"))))
  (`CorrbolgInventoryComponent.RequestAction` (`self.ACOMP_CorrbolgSampleInventory`) (`BlueprintGameplayTagLibrary.MakeLiteralGameplayTag` (struct :`TagName` "Corrbolg.Inventory.Action.Log")) _returnvalue_3))

(event `RetrieveItem`
  (bind _returnvalue (`BlueprintInstancedStructLibrary.MakeInstancedStruct` (make `CorrbolgStorageContextFragment` (`KismetArrayLibrary.Array_Random` (`|MakeArray` "/Game/Fragments/DA_Apple.DA_Apple" "/Game/Fragments/DA_Milk.DA_Milk" "/Game/Fragments/DA_Orange.DA_Orange" "/Game/Fragments/DA_Tea.DA_Tea" :!type "CorrbolgItemDefinition Object Reference")) 1)))
  (`CorrbolgInventoryComponent.RequestAction` (`self.ACOMP_CorrbolgSampleInventory`) (`BlueprintGameplayTagLibrary.MakeLiteralGameplayTag` (struct :`TagName` "Corrbolg.Inventory.Action.Retrieve")) _returnvalue)
  (goto _label))

(fn `UserConstructionScript`)